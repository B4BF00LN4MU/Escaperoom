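; BP_Gimmick is an escape room gimmick that tracks quest completion through an IsComplete flag.
; EventQuestComplete sets that flag, while BeginPlay fetches DT_ItemTable row names without using them.
; OnCheckQuest takes an item struct and tests its ItemType, but does nothing with the result.
; Disconnected nodes for removing a matched item and fetching a player pawn component suggest an unfinished item check.
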(event EventBeginPlay
  (DataTable|GetDataTableRowNames "/Game/EscapeRoom/Data/DT_ItemTable.DT_ItemTable"))

(fn ConstructionScript)

(fn OnCheckQuest
  (params (ST_Item :type ST%20Item%20Structure))
  (if (== (.ItemType (Utilities|Struct|BreakST_Item ST_Item)) 0)
    _))

(fn EventQuestComplete
  (Variables|Default|SetIsComplete true))