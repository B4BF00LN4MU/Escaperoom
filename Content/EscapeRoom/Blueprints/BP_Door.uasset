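; Escape room door actor that swings its SMDoor mesh open automatically on BeginPlay.
; DoOpenDoor plays a timeline whose RotationZ track, scaled by -90, drives the mesh's relative yaw, and DoCloseDoor plays it in reverse from the end.
; A separate UpdateOpeningDoor function eases yaw toward -90 with FInterpTo and clears its own timer on arrival, but nothing in this Blueprint starts that timer.
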(event Custom|DoCloseDoor
  (bind _rotationz (Timeline|Timeline ReverseFromEnd)
    (:Update
      (Transformation|SetRelativeRotation (Variables|Default|GetSM_Door) (Math|Rotator|MakeRotator 0.0 0.0 (* _rotationz -9e+01)) false false))))

(event Custom|DoOpenDoor
  (bind _rotationz (Timeline|Timeline PlayFromStart)
    (:Update
      (Transformation|SetRelativeRotation (Variables|Default|GetSM_Door) (Math|Rotator|MakeRotator 0.0 0.0 (* _rotationz -9e+01)) false false))))

(event EventBeginPlay
  (CallFunction|DoOpenDoor))

(fn ConstructionScript)

(fn UpdateOpeningDoor
  (bind _sm_door (Variables|Default|GetSM_Door))
  (bind _relativerotation (Variables|/Script/Engine.SceneComponent|GetRelativeRotation _sm_door))
  (bind _returnvalue (Math|Interpolation|FInterpTo (.yaw _relativerotation) -9e+01 0.01 1e+01))
  (Transformation|SetRelativeRotation _sm_door (Math|Rotator|MakeRotator 0.0 0.0 _returnvalue) false false)
  (if (Math|Float|NearlyEqual(Float) _returnvalue -9e+01 1e-06)
    (Transformation|SetRelativeRotation (Variables|Default|GetSM_Door) "0.000000,-90.000000,0.000000" false false)
    (Utilities|Time|ClearTimerbyFunctionName 0 "UpdateOpeningDoor")))