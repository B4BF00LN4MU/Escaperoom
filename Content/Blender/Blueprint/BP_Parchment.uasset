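; BP_Parchment is a Blueprint for a parchment that appears with a steam effect when its Box trigger is overlapped.
; The three parchment components and the PSteamLit effect start hidden on BeginPlay.
; Any overlap shows the steam at once and starts two named timers, one revealing the parchment pieces and a later one hiding the steam.
; The parchment is never hidden again, and the overlap has no filter or one-shot guard.
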(event OnComponentBeginOverlap(Box)
  (params (OverlappedComponent :type Primitive%20Component%20Object%20Reference) (OtherActor :type Actor%20Object%20Reference) (OtherComp :type Primitive%20Component%20Object%20Reference) (OtherBodyIndex :type Integer) (bFromSweep :type Boolean) (SweepResult :type Hit%20Result%20Structure%20%28by%20ref%29))
  (Rendering|SetVisibility (Variables|Default|GetP_Steam_Lit) true false)
  (Utilities|Time|SetTimerbyFunctionName 0 "OnVisibilityParchment" 2.0)
  (Utilities|Time|SetTimerbyFunctionName 0 "OffVisibilityParticle" 4.0))

(event EventBeginPlay
  (Rendering|SetVisibility (Variables|Default|GetParchment) false false))

(fn ConstructionScript)

(fn OnVisibilityParchment
  (Rendering|SetVisibility (Variables|Default|GetParchment) true false))

(fn OffVisibilityParticle
  (Rendering|SetVisibility (Variables|Default|GetP_Steam_Lit) false false))